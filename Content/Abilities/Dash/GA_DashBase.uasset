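; GA_DashBase is a base Gameplay Ability that dashes the avatar using a constant root motion force.
; On activation it commits the ability, then applies the force along its Direction and Strength variables, maintaining the last root motion velocity afterward.
; When the force finishes, it force-commits the cooldown, ends the ability and prints a debug message.
; A failed commit ends the ability immediately.
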(event `self.K2_ActivateAbility`
  (bind _returnvalue (`self.K2_CommitAbility`))
  (if _returnvalue
    (`AbilityTask_ApplyRootMotionConstantForce.ApplyRootMotionConstantForce` "None" (`self.Direction`) (`self.Strength`) 0.0 false null "MaintainLastRootMotionVelocity" (`Actor.GetVelocity` (`self.GetAvatarActorFromActorInfo`))
      (:`OnFinish`
        (`self.K2_CommitAbilityCooldown` false true)
        (`self.K2_EndAbility`)
        (`KismetSystemLibrary.PrintString` "In CD")))
    (else
      (`self.K2_EndAbility`))))