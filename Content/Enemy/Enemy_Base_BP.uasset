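; Enemy_Base_BP is an enemy pawn that hunts the player and restarts the level when it reaches them.
; Three seconds after play begins, it starts an AI move toward the player character.
; On success it waits briefly, prints a caught message and runs the restartlevel console command.
; On failure it retries the chase after a short delay, forming a persistent pursuit loop.
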(event `self.ReceiveBeginPlay`
  (`KismetSystemLibrary.Delay` 3.0)
  (`self.Chase Player`))

(event `Chase Player`
  (`|AIMoveTo` self (0.0 0.0 0.0) (`GameplayStatics.GetPlayerCharacter` 0) 150.0
    (:`OnSuccess`
      (`KismetSystemLibrary.Delay` 0.5)
      (`KismetSystemLibrary.PrintString` "got caught, restart")
      (`KismetSystemLibrary.ExecuteConsoleCommand` "restartlevel" null))
    (:`OnFail`
      (`KismetSystemLibrary.Delay` 0.5)
      (`self.Chase Player`))))

(fn `UserConstructionScript`)